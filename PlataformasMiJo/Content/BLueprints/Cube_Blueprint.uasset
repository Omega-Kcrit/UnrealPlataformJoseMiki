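; Cube_Blueprint is a vertical sliding door that rises while opening and lowers otherwise.
; Actor begin and end overlap events set the Abriendose flag, with no filter on the overlapping actor.
; Each Tick calls SubirPuerta or BajaPuerta, moving the static mesh along world Z at a fixed, frame-rate-independent speed until it passes AlturaFinal or AlturaInicial.
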(event `self.ReceiveActorEndOverlap`
  (params (OtherActor :type "Actor Object Reference"))
  (set `self.Abriendose` false))

(event `self.ReceiveActorBeginOverlap`
  (params (OtherActor :type "Actor Object Reference"))
  (set `self.Abriendose` true))

(event `self.ReceiveTick`
  (params (DeltaSeconds :type "Float (single-precision)"))
  (if (`self.Abriendose`)
    (`self.Subir puerta` DeltaSeconds)
    (else
      (`self.Baja Puerta` DeltaSeconds))))

(fn `Baja Puerta`
  (params (DeltaTime :type "Float (double-precision)"))
  (bind (_returnvalue_x _returnvalue_y _returnvalue_z) (`KismetMathLibrary.BreakVector` (`SceneComponent.K2_GetComponentLocation` (`self.StaticMeshComponent`))))
  (bind (_returnvalue_x_2 _returnvalue_y_2 _returnvalue_z_2) (`KismetMathLibrary.BreakVector` (`SceneComponent.K2_GetComponentLocation` (`self.StaticMeshComponent`))))
  (if (not (<= _returnvalue_z (`self.Altura inicial`)))
    (`SceneComponent.K2_SetWorldLocation` (`self.StaticMeshComponent`) (`KismetMathLibrary.MakeVector` _returnvalue_x_2 _returnvalue_y_2 (- _returnvalue_z_2 (* DeltaTime 100.0))) false false)))

(fn `Subir puerta`
  (params (deltaTime :type "Float (double-precision)"))
  (bind (_returnvalue_x _returnvalue_y _returnvalue_z) (`KismetMathLibrary.BreakVector` (`SceneComponent.K2_GetComponentLocation` (`self.StaticMeshComponent`))))
  (if (not (<= (`self.Altura Final`) _returnvalue_z))
    (`SceneComponent.K2_SetWorldLocation` (`self.StaticMeshComponent`) (`KismetMathLibrary.MakeVector` _returnvalue_x _returnvalue_y (+ (* deltaTime 100.0) _returnvalue_z)) false false)))

(fn `UserConstructionScript`)