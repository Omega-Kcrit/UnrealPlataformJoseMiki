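; AI controller that drives an enemy through the AI_BT behavior tree, started on BeginPlay.
; AI Perception updates for FirstPersonCharacter write the sensed result to the CanSeePlayer blackboard key.
; An older patrol method that moved to random TargetPoints remains as unconnected logic, along with its GetRandomPoint helper.
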(event `self.ReceiveBeginPlay`
  (`self.RunBehaviorTree` "/Game/BLueprints/AI/AI_BT.AI_BT"))

(event `self.AIPerception.OnTargetPerceptionUpdated`
  (params (Actor :type "Actor Object Reference") (Stimulus :type "AIStimulus Structure"))
  (cast `/Game/FirstPersonBP/Blueprints/FirstPersonCharacter` Actor)
  (`BlackboardComponent.SetValueAsBool` (`AIBlueprintHelperLibrary.GetBlackboard` null) "CanSeePlayer" (`.bSuccessfullySensed` (break `AIStimulus` Stimulus))))

(fn `GetRandomPoint`
  (returns (RandomPoint :type "Actor Object Reference"))
  (bind _waypoints (`self.Waypoints`))
  (return (`|GetArrayItem` _waypoints (`KismetMathLibrary.RandomIntegerInRange` 0 (- (`KismetArrayLibrary.Array_Length` _waypoints) 1)))))

(fn `UserConstructionScript`)