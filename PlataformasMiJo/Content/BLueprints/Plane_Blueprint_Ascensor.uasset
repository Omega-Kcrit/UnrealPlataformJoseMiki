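; Elevator platform Blueprint that rises while an actor overlaps it and descends when the overlap ends.
; Overlap events toggle the Subiendose flag, and Tick calls SubirAscensor or BajarAscensor accordingly.
; Each function moves the static mesh vertically at a constant, frame-rate-independent speed until its world Z reaches AlturaFinal or AlturaInicial.
; Any actor triggers it, and a single end overlap starts the descent even if others remain.
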(event `self.ReceiveActorEndOverlap`
  (params (OtherActor :type "Actor Object Reference"))
  (set `self.Subiendose` false))

(event `self.ReceiveActorBeginOverlap`
  (params (OtherActor :type "Actor Object Reference"))
  (set `self.Subiendose` true))

(event `self.ReceiveTick`
  (params (DeltaSeconds :type "Float (single-precision)"))
  (if (`self.Subiendose`)
    (`self.Subir Ascensor` DeltaSeconds)
    (else
      (`self.Bajar Ascensor` DeltaSeconds))))

(fn `Bajar Ascensor`
  (params (DeltaTime :type "Float (double-precision)"))
  (bind (_returnvalue_x _returnvalue_y _returnvalue_z) (`KismetMathLibrary.BreakVector` (`SceneComponent.K2_GetComponentLocation` (`self.StaticMeshComponent`))))
  (if (not (<= _returnvalue_z (`self.Altura Inicial`)))
    (`SceneComponent.K2_SetWorldLocation` (`self.StaticMeshComponent`) (`KismetMathLibrary.MakeVector` _returnvalue_x _returnvalue_y (- _returnvalue_z (* DeltaTime 100.0))) false false)))

(fn `Subir Ascensor`
  (params (DeltaTime :type "Float (double-precision)"))
  (bind (_returnvalue_x _returnvalue_y _returnvalue_z) (`KismetMathLibrary.BreakVector` (`SceneComponent.K2_GetComponentLocation` (`self.StaticMeshComponent`))))
  (if (not (<= (`self.Altura final`) _returnvalue_z))
    (`SceneComponent.K2_SetWorldLocation` (`self.StaticMeshComponent`) (`KismetMathLibrary.MakeVector` _returnvalue_x _returnvalue_y (+ (* DeltaTime 100.0) _returnvalue_z)) false false)))

(fn `UserConstructionScript`)