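; Door actor that slides up when an actor overlaps it, optionally costing one key or a coin amount shown on its text label.
; Overlap spends from ThirdPersonCharacter's counters, or from ThirdPersonGameMode's for any other actor (first-person path, with sound on payment), and permanently clears that requirement.
; Tick moves the mesh toward AlturaFinal while the open flag is set, lowering it to AlturaInicial after overlap ends.
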(event `self.ReceiveBeginPlay`
  (if (`self.RequiereLlave`)
    (`TextRenderComponent.K2_SetText` (`self.DoorDesc`) (`KismetTextLibrary.Conv_StringToText` "Hacen falta 1 llave"))
    (elif (`self.Requiere Coins`)
      (`TextRenderComponent.K2_SetText` (`self.DoorDesc`) (`KismetTextLibrary.Conv_StringToText` (`KismetStringLibrary.Concat_StrStr` (`KismetTextLibrary.Conv_TextToString` (`KismetTextLibrary.Conv_StringToText` "Requiere Coins: ")) (`KismetStringLibrary.Conv_IntToString` (`self.CoinsReq`)))))
      (else
        (`TextRenderComponent.K2_SetText` (`self.DoorDesc`) (`KismetTextLibrary.Conv_StringToText` "No hace falta nada"))))))

(event `self.ReceiveActorEndOverlap`
  (params (OtherActor :type "Actor Object Reference"))
  (set `self.Abriendose` false))

(event `self.ReceiveActorBeginOverlap`
  (params (OtherActor :type "Actor Object Reference"))
  (bind _returnvalue (`self.K2_GetActorLocation`))
  (bind _coinsreq (`self.CoinsReq`))
  (bind _coinsreq_2 (`self.CoinsReq`))
  (bind _asthird_person_game_mode (cast `/Game/ThirdPersonBP/Blueprints/ThirdPersonGameMode` (`GameplayStatics.GetGameMode`) :!pure true))
  (bind _coins (`/Game/ThirdPersonBP/Blueprints/ThirdPersonGameMode.Coins` _asthird_person_game_mode))
  (bind _keys (`/Game/ThirdPersonBP/Blueprints/ThirdPersonGameMode.Keys` _asthird_person_game_mode))
  (cast `/Game/ThirdPersonBP/Blueprints/ThirdPersonCharacter` OtherActor
    (:`then`
      ;[1 1 1] Third Person
      (if (`self.RequiereLlave`)
        (bind _asthird_person_character (cast `/Game/ThirdPersonBP/Blueprints/ThirdPersonCharacter` OtherActor))
        (bind _keys_2 (`/Game/ThirdPersonBP/Blueprints/ThirdPersonCharacter.Keys` _asthird_person_character))
        (if (> _keys_2 0)
          (set `/Game/ThirdPersonBP/Blueprints/ThirdPersonCharacter.Keys` (- _keys_2 1) _asthird_person_character)
          (set `self.Abriendose` true)
          (set `self.RequiereLlave` false))
        (elif (`self.Requiere Coins`)
          (bind _asthird_person_character_2 (cast `/Game/ThirdPersonBP/Blueprints/ThirdPersonCharacter` OtherActor))
          (bind _coins_2 (`/Game/ThirdPersonBP/Blueprints/ThirdPersonCharacter.Coins` _asthird_person_character_2))
          (if (>= _coins_2 _coinsreq)
            (set `/Game/ThirdPersonBP/Blueprints/ThirdPersonCharacter.Coins` (- _coins_2 _coinsreq) _asthird_person_character_2)
            (set `self.Abriendose` true)
            (set `self.Requiere Coins` false))
          (else
            (set `self.Abriendose` true)))))
    (:`CastFailed`
      ;[1 1 1] First Person
      (if (`self.RequiereLlave`)
        (if (> _keys 0)
          (set `/Game/ThirdPersonBP/Blueprints/ThirdPersonGameMode.Keys` (- _keys 1) _asthird_person_game_mode)
          (`GameplayStatics.PlaySoundAtLocation` "/Game/Sounds/door_open.door_open" _returnvalue (struct) 1.0 1.0 0.0 null null null)
          (set `self.Abriendose` true)
          (set `self.RequiereLlave` false))
        (elif (`self.Requiere Coins`)
          (if (>= _coins _coinsreq_2)
            (set `/Game/ThirdPersonBP/Blueprints/ThirdPersonGameMode.Coins` (- _coins _coinsreq_2) _asthird_person_game_mode)
            (`GameplayStatics.PlaySoundAtLocation` "/Game/Sounds/door_open.door_open" _returnvalue (struct) 1.0 1.0 0.0 null null null)
            (set `self.Abriendose` true)
            (set `self.Requiere Coins` false))
          (else
            (set `self.Abriendose` true)))))))

(event `self.ReceiveTick`
  (params (DeltaSeconds :type "Float (single-precision)"))
  (if (`self.Abriendose`)
    (`self.Subir puerta` DeltaSeconds)
    (else
      (`self.Baja Puerta` DeltaSeconds))))

(fn `Baja Puerta`
  (params (DeltaTime :type "Float (double-precision)"))
  (bind (_returnvalue_x _returnvalue_y _returnvalue_z) (`KismetMathLibrary.BreakVector` (`SceneComponent.K2_GetComponentLocation` (`self.StaticMeshComponent`))))
  (bind (_returnvalue_x_2 _returnvalue_y_2 _returnvalue_z_2) (`KismetMathLibrary.BreakVector` (`SceneComponent.K2_GetComponentLocation` (`self.StaticMeshComponent`))))
  (if (not (<= _returnvalue_z (`self.Altura inicial`)))
    (`SceneComponent.K2_SetWorldLocation` (`self.StaticMeshComponent`) (`KismetMathLibrary.MakeVector` _returnvalue_x_2 _returnvalue_y_2 (- _returnvalue_z_2 (* DeltaTime 100.0))) false false)))

(fn `Subir puerta`
  (params (deltaTime :type "Float (double-precision)"))
  (bind (_returnvalue_x _returnvalue_y _returnvalue_z) (`KismetMathLibrary.BreakVector` (`SceneComponent.K2_GetComponentLocation` (`self.StaticMeshComponent`))))
  (if (not (<= (`self.Altura Final`) _returnvalue_z))
    (`SceneComponent.K2_SetWorldLocation` (`self.StaticMeshComponent`) (`KismetMathLibrary.MakeVector` _returnvalue_x _returnvalue_y (+ (* deltaTime 100.0) _returnvalue_z)) false false)))

(fn `UserConstructionScript`)